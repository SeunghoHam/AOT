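; Networked first-person player character with dual grappling hooks, a weapon, crouch, run toggle, interaction, mine placement and camera possession.
; Grapple events drive the SCGH component, while a per-tick camera trace sets the can-grapple flag.
; Local control selects arm or body mesh for display and weapon attachment, and authority caches control rotation for non-local reads.
; Death ragdolls the body, drops the gun, moves the camera to the head and notifies the GameMode.
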(event `self.ReceiveTick`
  (params (DeltaSeconds :type "Float (single-precision)"))
  (bind _returnvalue (`GameplayStatics.GetPlayerCameraManager` 0))
  (bind _returnvalue_2 (`self.K2_GetActorLocation` _returnvalue))
  (`|ExecutionSequence`
    (:`then_0`
      ;[1 1 1] UI 변경시키는 LineTrace
      (bind _outhit (`KismetSystemLibrary.LineTraceSingle` :`Start` _returnvalue_2 :`End` (+ _returnvalue_2 (* (`self.GetActorForwardVector` _returnvalue) (`/Game/SC_GH/SC_GH.DistanceFire` (`self.SC_GH`)))) :`TraceChannel` "TraceTypeQuery1" :`DrawTime` 0.0))
      (if (`GameplayStatics.BreakHitResult` _outhit)
        (set `self.IsCanGrapping` true)
        (else
          (set `self.IsCanGrapping` false))))
    (:`then_1`
      (`/Engine/EditorBlueprintResources/ActorMacros.Switch Has Authority`
        (:`Authority`
          (set `self.SimulatedControlRotation` (`self.GetControlRotation`)))))))

(event `self.ReceiveBeginPlay`
  (`/Engine/EditorBlueprintResources/ActorMacros.Switch Has Authority`
    (:`Authority`
      (set `self.SimulatedControlRotation` (struct)))))

(event `self.OnSetupWeapon`
  (bind _arm_mesh (`self.Arm Mesh`))
  (bind _mesh (`self.Mesh`))
  (bind _weaponactor (`self.WeaponActor`))
  (if (`self.IsLocallyControlled`) :!label _label
    (`/Engine/EditorBlueprintResources/StandardMacros.IsValid` (`self.WeaponActor`)
      (:`Is Valid`
        ;[1 1 1] ArmMesh의 R_GunSocket
        (`self.K2_AttachToComponent` _weaponactor (`self.Arm Mesh`) "R_GunSocket" "SnapToTarget" "SnapToTarget" "KeepRelative" true))
      (:`Is Not Valid`
        _))
    (`SceneComponent.SetVisibility` _mesh false false)
    (`SceneComponent.SetVisibility` _arm_mesh true true)
    (else
      (`/Engine/EditorBlueprintResources/StandardMacros.IsValid` (`self.WeaponActor`)
        (:`Is Valid`
          ;[1 1 1] Mesh의 R_GunSocket
          (`self.K2_AttachToComponent` _weaponactor (`self.Mesh`) "R_GunSocket" "SnapToTarget" "SnapToTarget" "KeepRelative" true))
        (:`Is Not Valid`
          _))
      (`SceneComponent.SetVisibility` _mesh true false)
      (`SceneComponent.SetVisibility` _arm_mesh false true))))

(event `self.ReceivePossessed`
  (params (NewController :type "Controller Object Reference"))
  (goto _label))

(event `OnCrouch`
  (`self.Crouch`))

(event `self.ReceiveUnpossessed`
  (params (OldController :type "Controller Object Reference"))
  (goto _label))

(event `ServerUpdateCrouch`
  (`self.OnCrouch`))

(event `ClientUpdateCrouch`
  (`self.ServerUpdateCrouch`))

(event `self.OnPressedGrappingR`
  (bind _sc_gh (`self.SC_GH`))
  (if (`/Game/SC_GH/SC_GH.usedR` _sc_gh)
    (`/Game/SC_GH/SC_GH.DetachCableR` _sc_gh)
    (else
      (set `/Game/SC_GH/SC_GH.Launch Speed` 0.0 _sc_gh)
      (`/Game/SC_GH/SC_GH.GrappingR` _sc_gh))))

(event `self.OnPressedHookMove`
  (bind _sc_gh (`self.SC_GH`))
  (if (<= (`KismetArrayLibrary.Array_Length` (`/Game/SC_GH/SC_GH.GrappleComponent` _sc_gh)) 1)
    (`/Game/SC_GH/SC_GH.DetachCable1` _sc_gh)
    (else
      (`/Game/SC_GH/SC_GH.DetachCable2` _sc_gh))))

(event `InputAction|Crouch`
  (params (Key :type "Key Structure"))
  (:`Pressed`
    (set `self.IsCrouching` true)
    (bind (_direction _crouch_alpha) (`Timeline|T_Crouching` :!label _label_2)
      (:`Update`
        (`CapsuleComponent.SetCapsuleHalfHeight` (`self.CapsuleComponent`) (`KismetMathLibrary.Lerp` 88.0 44.0 _crouch_alpha) true))))
  (:`Released`
    (set `self.IsCrouching` false)
    (goto _label_2 :!via `Reverse`)))

(event `self.OnPressedGrapping`)

(event `self.OnPressedGrappingL`
  (bind _sc_gh (`self.SC_GH`))
  (if (`/Game/SC_GH/SC_GH.usedL` _sc_gh)
    (`/Game/SC_GH/SC_GH.DetachCableL` _sc_gh)
    (else
      (set `/Game/SC_GH/SC_GH.Launch Speed` 0.0 _sc_gh)
      (`/Game/SC_GH/SC_GH.GrappingL` _sc_gh))))

(event `self.OnJump`)

(event `self.OnDie`
  (bind _weaponactor (`self.WeaponActor`))
  (bind _mesh (`self.Mesh`))
  (`|ExecutionSequence`
    (:`then_0`
      (`SceneComponent.SetVisibility` _mesh true true)
      (`PrimitiveComponent.SetSimulatePhysics` _mesh true)
      (`PrimitiveComponent.SetCollisionEnabled` _mesh "QueryAndPhysics")
      (`SceneComponent.SetVisibility` (`self.Arm Mesh`) false true)
      ;[1 1 1] 죽었을때 총기 해제 및 피직스 시뮬레이션 ...
      (`self.K2_DetachFromActor` _weaponactor "KeepWorld" "KeepWorld" "KeepWorld")
      (bind _asbp_m4a1 (cast `/Game/Blueprints/BP_M4A1` _weaponactor))
      (bind _skeletalmesh (`/Game/Blueprints/BP_M4A1.SkeletalMesh` _asbp_m4a1))
      (`PrimitiveComponent.SetSimulatePhysics` _skeletalmesh true)
      (`PrimitiveComponent.SetCollisionProfileName` _skeletalmesh "BlockAllDynamic" true))
    (:`then_1`
      (if (`self.IsLocallyControlled`)
        (`SceneComponent.K2_AttachToComponent` (`self.FPCamera`) (`self.Mesh`) "head" "SnapToTarget" "SnapToTarget" "KeepWorld" true)))
    (:`then_2`
      ;[1 1 1] 나 죽었다고 서버에 알려주기
      (if (`self.HasAuthority`)
        (bind _asbp_aotdefence_game_mode (cast `/Game/Blueprints/BP_AOTDefenceGameMode` (`GameplayStatics.GetGameMode`)))
        (bind _asaotplayer_state (cast `AOTPlayerState` (`Controller.PlayerState` (`self.GetController`))))
        (`/Game/Blueprints/BP_AOTDefenceGameMode.OnPlayerDead` _asbp_aotdefence_game_mode _asaotplayer_state)))))

(event `InputAction|Interact`
  (params (Key :type "Key Structure"))
  (bind _fpcamera (`self.FPCamera`))
  (bind _returnvalue (`SceneComponent.K2_GetComponentLocation` _fpcamera))
  ;[1 1 1] Interact Event - BPI_Interface
  (:`Pressed`
    (bind _outhit (`KismetSystemLibrary.SphereTraceSingle` :`Start` _returnvalue :`End` (+ _returnvalue (* (`SceneComponent.GetForwardVector` _fpcamera) 500.0)) :`Radius` 2.0 :`TraceChannel` "TraceTypeQuery1" :`DrawDebugType` "ForDuration"))
    (bind (_bblockinghit _binitialoverlap _time _distance _location _impactpoint _normal _impactnormal _physmat _hitactor) (`GameplayStatics.BreakHitResult` _outhit))
    (if _bblockinghit
      (if (`KismetSystemLibrary.DoesImplementInterface` _hitactor "/Game/Blueprints/Door/BPI_Interaction.BPI_Interaction_C")
        (message `/Game/Blueprints/Door/BPI_Interaction.Interact` _hitactor)))))

(event `InputAction|Run`
  (params (Key :type "Key Structure"))
  (bind _charactermovement (`self.CharacterMovement`))
  (:`Pressed`
    (`/Engine/EditorBlueprintResources/StandardMacros.FlipFlop`
      (:`A`
        (`KismetSystemLibrary.PrintString` "빨라지기")
        (set `CharacterMovementComponent.MaxWalkSpeed` 6000.0 _charactermovement))
      (:`B`
        (`KismetSystemLibrary.PrintString` "느려지기")
        (set `CharacterMovementComponent.MaxWalkSpeed` 600.0 _charactermovement)))))

(event `InputAction|Garget`
  (params (Key :type "Key Structure"))
  ;[1 1 1] 가젯 입력
  (:`Pressed`
    (`self.RequestSpawnMine`)))

(event `RequestSpawnMine`
  (bind (_outlocation _outrotation) (`self.GetActorEyesViewPoint`))
  (bind (_outhit _returnvalue) (`KismetSystemLibrary.LineTraceSingle` _outlocation (+ _outlocation (* (`KismetMathLibrary.Conv_RotatorToVector` _outrotation) 1000.0)) "TraceTypeQuery1"))
  (if _returnvalue
    (bind (_bblockinghit _binitialoverlap _time _distance _location _impactpoint _normal _impactnormal _physmat _hitactor) (`GameplayStatics.BreakHitResult` _outhit))
    (if (!= (`GameplayStatics.GetObjectClass` _hitactor) "/Script/Engine.Pawn")
      (`|SpawnActorFromClass` "/Game/Blueprints/Garget/BP_Mine.BP_Mine_C" (`KismetMathLibrary.MakeTransform` _impactpoint (`KismetMathLibrary.MakeRotFromZ` _impactnormal)) "Undefined" "OverrideRootScale" self null))))

(event `Key|Six`
  (params (Key :type "Key Structure"))
  (:`Pressed`
    (`self.UseCamera`)))

(event `UseCamera`
  ;[1 1 1] possess는 서버에서 이뤄저야 한다.
  (bind _outactors (`GameplayStatics.GetAllActorsOfClass` "/Script/BattleForces.Camera"))
  (if (> (`KismetArrayLibrary.Array_Length` _outactors) 0)
    (`Controller.Possess` (`self.GetController`) (`|GetArrayItem` _outactors))))

(fn `GetNetworkControlRotation`
  (returns (Rotation :type "Rotator Structure"))
  (return (select `bool` (`self.IsLocallyControlled`) :`false` (`self.SimulatedControlRotation`) :`true` (`self.GetControlRotation`))))

(fn `UserConstructionScript`)
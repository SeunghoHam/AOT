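; Player controller that sets the player's name, switches the player in and out of Camera gadgets, and shows in-game UI.
; BeginPlay sends the GameInstance's player name through the SetName console command.
; The gadget input calls a server event that exits a possessed Camera, or stops the pawn's movement and uses a random Camera in the level.
; ShowWidget swaps between waiting and in-game widgets on the local controller.
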(event `self.ReceiveBeginPlay`
  (bind _asbp_aotgame_instance (cast `/Game/Blueprints/BP_AOTGameInstance` (`GameplayStatics.GetGameInstance`)))
  (`KismetSystemLibrary.ExecuteConsoleCommand` (`KismetStringLibrary.Concat_StrStr` "SetName" (`/Game/Blueprints/BP_AOTGameInstance.PlayerName` _asbp_aotgame_instance)) self))

(event `InputAction|Garget`
  (params (Key :type "Key Structure"))
  (:`Pressed`
    (`self.ServerUseCameraGadget`)))

(event `ServerUseCameraGadget`
  (bind _returnvalue (`self.K2_GetPawn`))
  (bind _returnvalue_2 (`GameplayStatics.GetObjectClass` _returnvalue))
  (bind _ascamera (cast `Camera` _returnvalue)
    (:`then`
      (`Camera.UnusedGadget` _ascamera))
    (:`CastFailed`
      (if (not (or (== _returnvalue_2 "/Script/BattleForces.Camera") (`KismetMathLibrary.ClassIsChildOf` _returnvalue_2 "/Script/BattleForces.Camera")))
        (bind _outactors (`GameplayStatics.GetAllActorsOfClass` "/Script/BattleForces.Camera"))
        (if (> (`KismetArrayLibrary.Array_Length` _outactors) 0)
          ;[1 1 1] 클라이언트에서도 움직임이 멈추게 하는 함수
          (`MovementComponent.StopMovementImmediately` (`Pawn.GetMovementComponent` _returnvalue))
          (`Camera.UseGadget` (`KismetArrayLibrary.Array_Random` _outactors) self))))))

(fn `ShowWidget`
  (params (IsWaiting :type Boolean))
  (bind _showingwidget (`self.ShowingWidget`))
  (if (`self.IsLocalController`)
    (`/Engine/EditorBlueprintResources/StandardMacros.IsValid` _showingwidget
      (:`Is Valid`
        (`Widget.RemoveFromParent` _showingwidget))
      (:`Is Not Valid`
        _))
    (if IsWaiting
      (bind _returnvalue (`|CreateWidget` "/Game/Blueprints/Widget/WBP_InGameWaitingUI.WBP_InGameWaitingUI_C" self))
      (set `self.ShowingWidget` _returnvalue)
      (else
        (bind _returnvalue_2 (`|CreateWidget` "/Game/Blueprints/Widget/WBP_InGameUI.WBP_InGameUI_C" self))
        (set `self.ShowingWidget` _returnvalue_2)))
    (`UserWidget.AddToViewport` (`self.ShowingWidget`) 0)))

(fn `UserConstructionScript`)